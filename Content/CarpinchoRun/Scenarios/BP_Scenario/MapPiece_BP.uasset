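; Map piece for an endless runner that chains random segments ahead of the character and removes itself once passed.
; When the character enters its Box, it raises their capped movement speed and animation speed, then spawns a random PieceList entry at ArrowEnd.
; It prints the game mode's points without changing them, then destroys itself after a delay.
; RestartGame zeroes the stored character's animation speed and calls ResetLevel, which reopens the current level after a delay.
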(event `self.Box.OnComponentBeginOverlap`
  (params (OverlappedComponent :type "PrimitiveComponent Object Reference") (OtherActor :type "Actor Object Reference") (OtherComp :type "PrimitiveComponent Object Reference") (OtherBodyIndex :type Integer) (bFromSweep :type Boolean) (SweepResult :type "HitResult Structure (by ref)"))
  (bind _piecelist (`self.PieceList`))
  (bind _asbp_third_person_character (cast `/Game/ThirdPerson/Blueprints/BP_ThirdPersonCharacter` OtherActor))
  (set `self.BP_Character` _asbp_third_person_character)
  ;[0 0 0 0.568] Speed Up Character
  (set `/Game/ThirdPerson/Blueprints/BP_ThirdPersonCharacter.Speed` (`KismetMathLibrary.FClamp` (+ (`/Game/ThirdPerson/Blueprints/BP_ThirdPersonCharacter.Speed` _asbp_third_person_character) 0.05) 0.0 2.0) _asbp_third_person_character)
  ;[0 0 0 0.563] Speed Up Anim
  (set `/Game/ThirdPerson/Blueprints/BP_ThirdPersonCharacter.SpeedAnimation` (+ (`/Game/ThirdPerson/Blueprints/BP_ThirdPersonCharacter.SpeedAnimation` _asbp_third_person_character) 10.0) _asbp_third_person_character)
  ;[0 0 0 0.546] Spawn new Piece and Delete old
  (`|SpawnActorFromClass` (`|GetArrayItem` _piecelist (`KismetMathLibrary.RandomIntegerInRange` 0 (`KismetArrayLibrary.Array_LastIndex` _piecelist))) (`SceneComponent.K2_GetComponentToWorld` (`self.ArrowEnd`)) "Undefined" "OverrideRootScale" null null)
  (bind _asbp_third_person_game_mode (cast `/Game/ThirdPerson/Blueprints/BP_ThirdPersonGameMode` (`GameplayStatics.GetGameMode`)))
  (bind _output_get (set `/Game/ThirdPerson/Blueprints/BP_ThirdPersonGameMode.CurrentPoints` (`/Game/ThirdPerson/Blueprints/BP_ThirdPersonGameMode.CurrentPoints` _asbp_third_person_game_mode) _asbp_third_person_game_mode))
  (`KismetSystemLibrary.PrintString` (`KismetStringLibrary.Conv_IntToString` _output_get))
  (`KismetSystemLibrary.Delay` 10.0)
  (`self.K2_DestroyActor`))

(event `RestartGame`
  (bind _asbp_third_person_character (cast `/Game/ThirdPerson/Blueprints/BP_ThirdPersonCharacter` (`self.BP_Character`)))
  (`|ExecutionSequence`
    (:`then_0`
      (set `/Game/ThirdPerson/Blueprints/BP_ThirdPersonCharacter.SpeedAnimation` 0.0 _asbp_third_person_character)
      (`KismetSystemLibrary.Delay` 10.0)
      (bind _returnvalue (`GameplayStatics.GetCurrentLevelName` true))
      (`GameplayStatics.OpenLevel` (`KismetStringLibrary.Conv_StringToName` _returnvalue)))))

(fn `UserConstructionScript`)